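; BP_WizardState holds the wizard character's health and its counts of red, blue and green boxes.
; AddDamage and AddHeal skip when already dead, clamp CurHp to a fixed 0–100 range rather than MaxHp, then broadcast UpdateHp, plus Death at zero.
; Each box function increments its counter and fires a matching dispatcher, so listeners receive changes through events, with no Tick logic.
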(event EventBeginPlay)

(event EventTick
  (params (DeltaSeconds :type Float%20%28single-precision%29)))

(fn ConstructionScript)

(fn AddDamage
  (params (Damage :type Float%20%28double-precision%29))
  (if (not (CallFunction|IsDeath))
    (bind _output_get (Variables|Default|SetCurHp (Math|Float|Clamp(Float) (- (Variables|Default|GetCurHp) Damage) 0.0 1e+02)))
    (Default|CallEventDispatcherUpdateHp _output_get (Variables|Default|GetMaxHp))
    (if (<= (Variables|Default|GetCurHp) 0.0)
      (Default|CallEventDispatcherDeath))))

(fn AddHeal
  (params (Heal :type Float%20%28double-precision%29))
  (if (not (CallFunction|IsDeath))
    (bind _output_get (Variables|Default|SetCurHp (Math|Float|Clamp(Float) (+ (Variables|Default|GetCurHp) Heal) 0.0 1e+02)))
    (Default|CallEventDispatcherUpdateHp _output_get (Variables|Default|GetMaxHp))
    (if (<= (Variables|Default|GetCurHp) 0.0)
      (Default|CallEventDispatcherDeath))))

(fn IsDeath
  (return (<= (Variables|Default|GetCurHp) 0.0)))

(fn AddRedBox
  (bind _output_get (Variables|Default|SetRedBox (+ (Variables|Default|GetRedBox) 1)))
  (Default|CallEventDispatcherRedBox _output_get))

(fn AddBlueBox
  (bind _output_get (Variables|Default|SetBlueBox (+ (Variables|Default|GetBlueBox) 1)))
  (Default|CallEventDispatcherBlueBox _output_get))

(fn AddGreenBox
  (bind _output_get (Variables|Default|SetGreenBox (+ (Variables|Default|GetGreenBox) 1)))
  (Default|CallEventDispatcherGreenBox _output_get))